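; Base interactable note actor that shows its text in the player HUD's note widget when interacted with.
; On BeginPlay it caches the first-person character and retries on a looping timer until that character's HUD is valid.
; Interaction sets and reveals the note widget, with flags for one-time use and self-destruction.
; It can also unlock another actor by making it interactable, chaining interactions together.
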(event Custom|SetHUD
  (Utilities|IsValid (Variables|/Game/FirstPerson/Blueprints/BP_FirstPersonCharacter.BP_FirstPersonCharacter_C|GetHUD (stale EventBeginPlay _asbp_first_person_character))
    (:Is%20Valid
      (Variables|Default|SetHUD (Variables|/Game/FirstPerson/Blueprints/BP_FirstPersonCharacter.BP_FirstPersonCharacter_C|GetHUD (stale EventBeginPlay _asbp_first_person_character)))
      (Utilities|Time|ClearandInvalidateTimerbyHandle (Variables|Default|GetHUDTimerHandle)))
    (:Is%20Not%20Valid
      (bind _returnvalue (Utilities|Time|SetTimerbyEvent (delegate Custom|SetHUD) 0.1 true))
      (Variables|Default|SetHUDTimerHandle _returnvalue))))

(event EventBeginPlay
  (|CallParentFunction)
  (Variables|Default|SetCanBeInteracted true)
  (bind _asbp_first_person_character (Utilities|Casting|CastToBP_FirstPersonCharacter (Game|GetPlayerCharacter 0)))
  (Utilities|IsValid (Variables|/Game/FirstPerson/Blueprints/BP_FirstPersonCharacter.BP_FirstPersonCharacter_C|GetHUD _asbp_first_person_character)
    (:Is%20Valid
      (Variables|Default|SetHUD (Variables|/Game/FirstPerson/Blueprints/BP_FirstPersonCharacter.BP_FirstPersonCharacter_C|GetHUD _asbp_first_person_character))
      (Utilities|Time|ClearandInvalidateTimerbyHandle (Variables|Default|GetHUDTimerHandle)))
    (:Is%20Not%20Valid
      (bind _returnvalue (Utilities|Time|SetTimerbyEvent (delegate Custom|SetHUD) 0.1 true))
      (Variables|Default|SetHUDTimerHandle _returnvalue))))

(event Collision|EventActorBeginOverlap
  (params (OtherActor :type Actor%20Object%20Reference))
  (|CallParentFunction OtherActor) ; This node is disabled and will not be called.\nDrag off pins to build functionality.
)

(event EventTick
  (params (DeltaSeconds :type Float%20%28single-precision%29))
  (|CallParentFunction DeltaSeconds) ; This node is disabled and will not be called.\nDrag off pins to build functionality.
)

(event EventActorInteracted
  (bind _actortounlock (Variables|Default|GetActorToUnlock))
  (bind _hud (Variables|Default|GetHUD))
  (bind _wb_note (Variables|/Game/CustomActors/WB_MainHUD.WB_MainHUD_C|GetWB_Note _hud))
  (if (Variables|Default|GetShouldInteractOnce)
    (Utilities|FlowControl|DoOnce false
      (:Completed
        _)))
  (Variables|/Game/CustomActors/WB_Note.WB_Note_C|SetDisplayedText _wb_note (Variables|Default|GetDisplayed%20Text))
  (Widget|SetVisibility _wb_note "Visible")
  (if (Variables|Default|GetShouldBeDestroyed)
    (Actor|DestroyActor))
  (Utilities|IsValid _actortounlock
    (:Is%20Valid
      (Variables|/Game/CustomActors/BP_InteractableActor_Base.BP_InteractableActor_Base_C|SetCanBeInteracted _actortounlock true))))

(fn ConstructionScript
  (|CallParentFunction))