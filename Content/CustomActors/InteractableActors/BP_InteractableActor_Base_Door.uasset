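; Base Blueprint for an interactable door that swings open once when the player interacts with it.
; ActorInteracted passes a DoOnce gate and plays a timeline that lerps the static mesh's relative yaw from zero to EndRotation.
; Roll and pitch are taken from the actor's rotation, and CanBeInteracted is cleared when the timeline finishes.
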(event EventBeginPlay
  (|CallParentFunction) ; This node is disabled and will not be called.\nDrag off pins to build functionality.
)

(event Collision|EventActorBeginOverlap
  (params (OtherActor :type Actor%20Object%20Reference))
  (|CallParentFunction OtherActor) ; This node is disabled and will not be called.\nDrag off pins to build functionality.
)

(event EventTick
  (params (DeltaSeconds :type Float%20%28single-precision%29))
  (|CallParentFunction DeltaSeconds) ; This node is disabled and will not be called.\nDrag off pins to build functionality.
)

(event EventActorInteracted
  (bind _returnvalue (Transformation|GetActorRotation))
  (Utilities|FlowControl|DoOnce false
    (:Completed
      (bind _newtrack_0 (Timeline|Timeline PlayFromStart)
        (:Update
          (Transformation|SetRelativeRotation (Variables|Default|GetStaticMesh) (Math|Rotator|MakeRotator (.roll _returnvalue) (.pitch _returnvalue) (Math|Float|Lerp 0.0 (Variables|Default|GetEndRotation) _newtrack_0)) false false))
        (:Finished
          (Variables|Default|SetCanBeInteracted false))))))

(fn ConstructionScript
  (|CallParentFunction))