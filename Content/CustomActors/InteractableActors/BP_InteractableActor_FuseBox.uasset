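; BP_InteractableActor_FuseBox is an interactable fuse box that switches on lighting when the player uses it.
; On ActorInteracted, it loops over arrays of cubes, clothing store lamps and other lamps, swapping a material slot specific to each group to MI_Emissive.
; It also makes every light in PointLightsArray visible.
; The change is one-way, with no toggle or off state in this Blueprint.
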(event EventBeginPlay
  (|CallParentFunction) ; This node is disabled and will not be called.\nDrag off pins to build functionality.
)

(event Collision|EventActorBeginOverlap
  (params (OtherActor :type Actor%20Object%20Reference))
  (|CallParentFunction OtherActor) ; This node is disabled and will not be called.\nDrag off pins to build functionality.
)

(event EventTick
  (params (DeltaSeconds :type Float%20%28single-precision%29))
  (|CallParentFunction DeltaSeconds) ; This node is disabled and will not be called.\nDrag off pins to build functionality.
)

(event EventActorInteracted
  (Utilities|FlowControl|Sequence
    (:then_0
      (for _array_element (Variables|Default|GetCubesArray)
        (Rendering|Material|SetMaterial (Variables|/Script/Engine.StaticMeshActor|GetStaticMeshComponent _array_element) 0 "/Game/CustomMaterials/MI_Emissive.MI_Emissive")))
    (:then_1
      (for _array_element_2 (Variables|Default|GetPointLightsArray)
        (Rendering|SetVisibility (Variables|/Script/Engine.PointLight|GetPointLightComponent _array_element_2) true false)))
    (:then_2
      (for _array_element_3 (Variables|Default|GetClothingStoreLampsArray)
        (Rendering|Material|SetMaterial (Variables|/Script/Engine.StaticMeshActor|GetStaticMeshComponent _array_element_3) 1 "/Game/CustomMaterials/MI_Emissive.MI_Emissive")))
    (:then_3
      (for _array_element_4 (Variables|Default|GetOtherLampsArray)
        (Rendering|Material|SetMaterial (Variables|/Script/Engine.StaticMeshActor|GetStaticMeshComponent _array_element_4) 2 "/Game/CustomMaterials/MI_Emissive.MI_Emissive")))))

(fn ConstructionScript
  (|CallParentFunction))